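; Main player controller Blueprint that adds animated transitions to showing and removing the pause menu.
; It extends the parent's DisplayPauseMenu and RemovePauseMenu events, casting the PauseMenu widget to BP_PauseMenu to reach its animation.
; Display plays that animation forward, while removal plays it in reverse and hides the widget after a short fixed delay.
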(event `self.DisplayPauseMenu`
  (`parent.DisplayPauseMenu`)
  (bind _asbp_pause_menu (cast `/Game/HUD/BP_PauseMenu` (`self.PauseMenu`)))
  (`UserWidget.PlayAnimation` _asbp_pause_menu (`/Game/HUD/BP_PauseMenu.PauseMenuAnimation` _asbp_pause_menu) 0.0 1 "Forward" 1.0 false))

(event `self.RemovePauseMenu`
  (`parent.RemovePauseMenu`)
  (bind _asbp_pause_menu (cast `/Game/HUD/BP_PauseMenu` (`self.PauseMenu`)))
  (`UserWidget.PlayAnimation` _asbp_pause_menu (`/Game/HUD/BP_PauseMenu.PauseMenuAnimation` _asbp_pause_menu) 0.0 1 "Reverse" 1.0 false)
  (`KismetSystemLibrary.Delay` 0.25)
  (`Widget.SetVisibility` (`self.PauseMenu`) "Hidden"))

(fn `UserConstructionScript`)